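; Playable character Blueprint that carries a gun and handles firing, weapon switching and death.
; On BeginPlay it spawns and attaches a temporary Gun_BP and caches the GameCamera.
; Keyboard and gamepad inputs drive the gun's trigger and shotgun or machinegun profiles, plus a debug player-index print.
; AffectHealth updates health and, on death, destroys the gun and sends the controller a despawn-on-kill message; screen-bounds debug logic is left unwired.
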(event `self.ReceiveTick`
  (params (DeltaSeconds :type "Float (single-precision)")))

(event `self.ReceiveBeginPlay`
  ;[1 1 1] Spawn Gun TEMP - CHANGE TO C++ CLASS
  (bind _returnvalue (`|SpawnActorFromClass` "/Game/BP/Gun_BP.Gun_BP_C" (`SceneComponent.GetRelativeTransform` (`self.GunTemp`)) "AlwaysSpawn" "OverrideRootScale" self))
  (bind _output_get (set `self.GunReference` _returnvalue))
  (`self.K2_AttachToActor` _output_get self "None" "KeepRelative" "KeepRelative" "KeepRelative" true)
  ;[1 1 1] Get Game Camera
  (bind _outactors (`GameplayStatics.GetAllActorsOfClass` "/Game/BP/GameCamera.GameCamera_C"))
  (for _array_element _outactors
    (set `self.GameCameraRef` _array_element)))

(event `Key|Gamepad_DPad_Right`
  (params (Key :type "Key Structure" :default "AnyKey"))
  ;[1 1 1] Temp weapon switch
  (:`Pressed`
    (`/Game/BP/Gun_BP.ShotgunProfile` (`self.GunReference`) :!label _label)))

(event `Key|Two`
  (params (Key :type "Key Structure" :default "AnyKey"))
  ;[1 1 1] Temp weapon switch
  (:`Pressed`
    (goto _label)))

(event `Key|SpaceBar`
  (params (Key :type "Key Structure" :default "AnyKey"))
  (bind _gunreference (`self.GunReference`))
  ;[1 1 1] Pull trigger
  (:`Pressed`
    (`/Game/BP/Gun_BP.PullTriggerBP` _gunreference :!label _label_2))
  (:`Released`
    (`/Game/BP/Gun_BP.ReleaseTriggerBP` _gunreference :!label _label_3)))

(event `Key|Tab`
  (params (Key :type "Key Structure" :default "AnyKey"))
  (:`Pressed`
    (bind _playerindex (`TurnBasedBlueprintLibrary.GetMyPlayerIndex` null "20" :!label _label_4))
    (`KismetSystemLibrary.PrintString` (`KismetStringLibrary.Conv_IntToString` _playerindex))))

(event `Key|Gamepad_DPad_Up`
  (params (Key :type "Key Structure" :default "AnyKey"))
  (:`Pressed`
    (goto _label_4)))

(event `Key|Gamepad_RightTrigger`
  (params (Key :type "Key Structure" :default "AnyKey"))
  ;[1 1 1] Pull trigger
  (:`Pressed`
    (goto _label_2))
  (:`Released`
    (goto _label_3)))

(event `Key|Gamepad_DPad_Left`
  (params (Key :type "Key Structure" :default "AnyKey"))
  ;[1 1 1] Temp weapon switch
  (:`Pressed`
    (`/Game/BP/Gun_BP.Machinegun Profile` (`self.GunReference`) :!label _label_5)))

(event `Key|One`
  (params (Key :type "Key Structure" :default "AnyKey"))
  ;[1 1 1] Temp weapon switch
  (:`Pressed`
    (goto _label_5)))

(event `/Game/BP/iDamagable.AffectHealth`
  (params (Delta :type "Float (single-precision)"))
  (`self.CalculateHealth` Delta)
  (`KismetSystemLibrary.PrintString` (`KismetStringLibrary.Conv_DoubleToString` (`self.Health`)))
  (if (`self.IsDead`)
    (`self.K2_DestroyActor` (`self.GunReference`))
    (message `/Game/BP/iSpawnControl.DespawnOnKill` (`self.GetController`))))

(fn `UserConstructionScript`)