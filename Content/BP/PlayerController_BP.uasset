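; Player controller Blueprint for Cargo Carnage that lets each player spawn and despawn through input.
; E or gamepad Special Right asks the CargoCarnage game mode to spawn this controller's player; Q or Special Left asks it to despawn.
; A DespawnonKill event reuses the same despawn path.
; All spawn logic lives in the game mode, which receives this controller as the argument.
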(event `Key|E`
  (params (Key :type "Key Structure" :default "AnyKey"))
  (:`Pressed`
    (bind _ascargo_carnage_game_mode_base_bp (cast `/Game/BP/CargoCarnageGameModeBase_BP` (`GameplayStatics.GetGameMode`) :!label _label))
    (`/Game/BP/CargoCarnageGameModeBase_BP.SpawnPlayer` _ascargo_carnage_game_mode_base_bp self)))

(event `Key|Gamepad_Special_Right`
  (params (Key :type "Key Structure" :default "AnyKey"))
  (:`Pressed`
    (goto _label)))

(event `Key|Gamepad_Special_Left`
  (params (Key :type "Key Structure" :default "AnyKey"))
  (:`Pressed`
    (bind _ascargo_carnage_game_mode_base_bp (cast `/Game/BP/CargoCarnageGameModeBase_BP` (`GameplayStatics.GetGameMode`) :!label _label_2))
    (`/Game/BP/CargoCarnageGameModeBase_BP.DeSpawnPlayer` _ascargo_carnage_game_mode_base_bp self)))

(event `Key|Q`
  (params (Key :type "Key Structure" :default "AnyKey"))
  (:`Pressed`
    (goto _label_2)))

(event `/Game/BP/iSpawnControl.DespawnOnKill`
  (goto _label_2))

(fn `UserConstructionScript`)