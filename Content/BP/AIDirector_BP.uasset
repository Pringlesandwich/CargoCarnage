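; AI director that starts a sabotage enemy wave against a random ship system when play begins.
; BeginPlay caches all test spawners and ship systems, then SpawnWave messages a random spawner with a random system target and spawn amount.
; The random-delay repeat is unwired, so only one wave fires.
; Debug prints re-roll their random picks, so logged names can differ from actual targets.
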(event `self.ReceiveBeginPlay`
  ;[1 1 1] Get all spawners and systems - wait a random time then spawn wave
  (bind _outactors (`GameplayStatics.GetAllActorsOfClass` "/Game/BP/EnemySpawnerTest.EnemySpawnerTest_C"))
  (set `self.Spawner` _outactors)
  (bind _outactors_2 (`GameplayStatics.GetAllActorsOfClass` "/Game/BP/ShipSystem_BP.ShipSystem_BP_C"))
  (set `self.Systems` _outactors_2)
  (`self.SpawnWave`))

(event `SpawnWave`
  (bind _spawner (`self.Spawner`))
  (bind _systems (`self.Systems`))
  (bind _output (`|GetArrayItem` _spawner (`KismetMathLibrary.RandomIntegerInRange` 0 (- (`KismetArrayLibrary.Array_Length` _spawner) 1))))
  (bind _output_2 (`|GetArrayItem` _systems (`KismetMathLibrary.RandomIntegerInRange` 0 (- (`KismetArrayLibrary.Array_Length` _systems) 1))))
  (set `self.SpawnTarget` _output)
  (`KismetSystemLibrary.PrintString` (`KismetSystemLibrary.GetDisplayName` _output))
  (set `self.SystemTarget` _output_2)
  (`KismetSystemLibrary.PrintString` (`KismetSystemLibrary.GetDisplayName` _output_2))
  (message `/Game/BP/iAIDirected.SpawnController` (`self.SpawnTarget`) (`self.SystemTarget`) (`KismetMathLibrary.RandomIntegerInRange` 20 15) true))

(fn `UserConstructionScript`)