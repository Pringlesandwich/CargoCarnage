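; Projectile actor that damages whatever damageable actor it overlaps.
; On overlap it checks the other actor for the IDamagable interface and sends its damage through AffectHealthMessage, cut to a quarter for actors tagged Friendly.
; It then destroys itself, whether or not the actor hit was damageable.
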(event `self.ReceiveActorBeginOverlap`
  (params (OtherActor :type "Actor Object Reference"))
  ;[1 1 1] Collision triggers iDamage Interface
  (bind _output_get (set `self.ActorHit` OtherActor))
  (if (`KismetSystemLibrary.DoesImplementInterface` _output_get "/Game/BP/iDamagable.iDamagable_C")
    (if (not (`self.ActorHasTag` (`self.ActorHit`) "Friendly"))
      (message `/Game/BP/iDamagable.AffectHealth` (`self.ActorHit`) (`self.DamageBP`))
      (else
        ;;[1 1 1] Quarter damage to friendly units
        (message `/Game/BP/iDamagable.AffectHealth` (`self.ActorHit`) (/ (`self.DamageBP`) 4.0)))))
  (`self.K2_DestroyActor`))

(fn `UserConstructionScript`)