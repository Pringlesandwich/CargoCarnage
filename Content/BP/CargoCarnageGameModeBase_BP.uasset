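; Game mode for Cargo Carnage that creates local players and handles their spawning and despawning.
; BeginPlay caches all PlayerStarts and creates players until the count exceeds three.
; SpawnPlayer and DeSpawnPlayer replace the controlled pawn with a PlayableCharacter_BP or InitPawn respectively, then set the view to CameraVariable.
; Both take transforms from GetSpawnPoints, whose random PlayerStart lookup appears unconnected.
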(event `self.ReceiveBeginPlay`
  (bind _number_of_players (`self.Number Of Players`))
  (bind _outactors (`GameplayStatics.GetAllActorsOfClass` "/Script/Engine.PlayerStart"))
  (set `self.SpawnPoints` _outactors)
  (while (<= _number_of_players 3)
    (set `self.Number Of Players` (+ _number_of_players 1))
    (`GameplayStatics.CreatePlayer` -1)))

(event `SpawnPlayer`
  (params (PlayerController :type "PlayerController Object Reference"))
  (bind _returnvalue (`Controller.K2_GetPawn` PlayerController))
  (`/Engine/EditorBlueprintResources/StandardMacros.IsValid` _returnvalue
    (:`Is Valid`
      (`self.K2_DestroyActor` _returnvalue)
      (bind _returnvalue_2 (`|SpawnActorFromClass` "/Game/BP/PlayableCharacter_BP.PlayableCharacter_BP_C" (`self.GetSpawnPoints`) "Undefined" "OverrideRootScale"))
      (`Controller.Possess` PlayerController _returnvalue_2)
      (`PlayerController.SetViewTargetWithBlend` PlayerController (`self.Camera Variable`) 0.0 "VTBlend_Linear" 0.0 false))))

(event `DeSpawnPlayer`
  (params (PlayerController :type "PlayerController Object Reference"))
  (bind _returnvalue (`Controller.K2_GetPawn` PlayerController))
  (`/Engine/EditorBlueprintResources/StandardMacros.IsValid` _returnvalue
    (:`Is Valid`
      (`self.K2_DestroyActor` _returnvalue)
      (bind _returnvalue_2 (`|SpawnActorFromClass` "/Game/BP/InitPawn.InitPawn_C" (`self.GetSpawnPoints`) "Undefined" "OverrideRootScale"))
      (`Controller.Possess` PlayerController _returnvalue_2)
      (`PlayerController.SetViewTargetWithBlend` PlayerController (`self.Camera Variable`) 0.0 "VTBlend_Linear" 0.0 false))))

(fn `UserConstructionScript`)