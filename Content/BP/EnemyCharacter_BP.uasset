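; Enemy character Blueprint that either moves to sabotage a target system assigned by its spawner or chases the closest player.
; A looping half-second timer drives AI MoveTo, picking the nearest PlayableCharacter within aggro range when not sabotaging.
; Taking damage while sabotaging pulls it and nearby enemies off sabotage; otherwise it is destroyed if dead.
; Overlapping a player starts a repeating timer that deals damage through AffectHealth until overlap ends.
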(event `self.ReceiveBeginPlay`
  ;[1 1 1] Call Track player every .5 seconds (if more efficient than tick)
  (`KismetSystemLibrary.K2_SetTimer` null "Track Player" 0.5 true))

(event `/Game/BP/iAIDirected.SetTargetSystem`
  (params (TargetSystem :type "/Game/BP/ShipSystem_BP Object Reference") (IsSabotage :type Boolean))
  ;[1 1 1] called from Spawner after spawn
  (set `self.TargetSystem` TargetSystem)
  (set `self.bIsSabotaging` IsSabotage))

(event `Track Player`
  (if (`self.bIsSabotaging`)
    ;[1 1 1] MoveToTargetSystem
    (`|AIMoveTo` self (0.0 0.0 0.0) (`self.TargetSystem`))
    (else
      ;[1 1 1] Call GetClosetPlayer then move to them
      (`self.GetClosestPlayer`)
      (`|AIMoveTo` self (0.0 0.0 0.0) (`self.TargetActor`) 5.0))))

(event `GetClosestPlayer`
  ;[1 1 1] Get Closest player - compares distance to an array of Playable Characters
  (set `self.Distances` (`self.AggroRange`))
  (bind _outactors (`GameplayStatics.GetAllActorsOfClass` "/Game/BP/PlayableCharacter_BP.PlayableCharacter_BP_C"))
  (for _array_element _outactors
    (bind _returnvalue (`self.GetDistanceTo` _array_element self))
    (`/Engine/EditorBlueprintResources/StandardMacros.CompareFloat` _returnvalue (`self.Distances`)
      (:`<`
        (set `self.TargetActor` _array_element)
        (set `self.Distances` _returnvalue)))))

(event `/Game/BP/iDamagable.AffectHealth`
  (params (Delta :type "Float (single-precision)"))
  ;[1 1 1] Damage Via iDamage Interface - Called if shot by player
  (`self.CalculateHealth` Delta)
  (if (`self.bIsSabotaging`)
    ;[1 1 1] get all within a short distance and set their sabotage
    (bind _outactors (`GameplayStatics.GetAllActorsOfClass` "EnemyCharacter_BP_C"))
    (for _array_element _outactors
      (if (<= (`self.GetDistanceTo` _array_element) 200.0)
        (set `/Game/BP/EnemyCharacter_BP.bIsSabotaging` false _array_element)))
    (set `self.bIsSabotaging` false)
    (elif (`self.IsDead`)
      (`self.K2_DestroyActor`))))

(event `self.ReceiveActorBeginOverlap`
  (params (OtherActor :type "Actor Object Reference"))
  ;[1 1 1] If Collision box is on player then damage them per socond
  (bind _asplayable_character_bp (cast `/Game/BP/PlayableCharacter_BP` OtherActor))
  (set `self.PlayerableCharaters` _asplayable_character_bp)
  (`KismetSystemLibrary.K2_SetTimer` null "DamagePlayer" (/ 1.0 (`self.AttacksPerSecond`)) true))

(event `DamagePlayer`
  ;[1 1 1] If Collision box is on player then damage them per socond
  (`/Game/BP/PlayableCharacter_BP.AffectHealth` (`self.PlayerableCharaters`) (`self.Damage`)))

(event `self.ReceiveActorEndOverlap`
  (params (OtherActor :type "Actor Object Reference"))
  ;[1 1 1] If Collision box is on player then damage them per socond
  (if (== OtherActor (`self.PlayerableCharaters`))
    (`KismetSystemLibrary.K2_ClearTimer` null "DamagePlayer")))

(fn `UserConstructionScript`)