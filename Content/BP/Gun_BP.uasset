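; Gun Blueprint that spawns projectiles from a muzzle, with temporary machine gun and shotgun profiles; the machine gun loads on BeginPlay.
; Pulling the trigger fires immediately unless cooling down, while Tick starts or clears a looping timer at the profile's fire rate.
; Each projectile gets random yaw spread from AddInaccuracy and receives damage after spawning, which a comment flags as buggy.
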(event `Machinegun Profile`
  ;[1 1 1] TEMP SETUP! Change per gun
  (set `self.TriggerDown` false)
  (`KismetSystemLibrary.PrintString` "Machine Gun")
  (set `self.isOnCooldown` false)
  ;;[1 1 1] Machine Gun Profile
  (set `self.ProjectileAmountBP` 1 :!label _label)
  (set `self.AccuracyBP` 5.0) ; THIS NEEDS TO BE TAKEN AWAY FROM 100 TO CREATE A PERCENTAGE
  (set `self.RoundsPerSecondBP` 12.0)
  (set `self.BulletDamage` -40.0))

(event `self.ReceiveBeginPlay`
  (goto _label))

(event `ShotgunProfile`
  ;[1 1 1] TEMP SETUP! Change per gun
  (set `self.TriggerDown` false)
  (`KismetSystemLibrary.PrintString` "Shotgun")
  (set `self.isOnCooldown` false)
  ;;[1 1 1] Shotgun Profile
  (set `self.ProjectileAmountBP` 5)
  (set `self.AccuracyBP` 20.0)
  (set `self.RoundsPerSecondBP` 2.0)
  (set `self.BulletDamage` -30.0))

(event `PullTriggerBP`
  ;[1 1 1] Press and release trigger - called by player
  (set `self.TriggerDown` true)
  (if (not (`self.isOnCooldown`))
    (`self.FireBP`)))

(event `ReleaseTriggerBP`
  ;[1 1 1] Press and release trigger - called by player
  (set `self.TriggerDown` false)
  (`self.Cooldown`))

(event `self.ReceiveTick`
  (params (DeltaSeconds :type "Float (single-precision)"))
  ;[1 1 1] Tick - Fire at rounds per second - TODO - make it work so player cant spam trigger
  (set `self.TransformTemp` (`SceneComponent.K2_GetComponentToWorld` (`self.MuzzleLocation`)))
  (if (`self.TriggerDown`)
    (`/Engine/EditorBlueprintResources/StandardMacros.DoOnce` false :!label _label_2
      (:`Completed`
        (`KismetSystemLibrary.K2_SetTimer` null "FireBP" (/ 1.0 (`self.RoundsPerSecondBP`)) true)
        (`self.Cooldown`)))
    (else
      (`KismetSystemLibrary.K2_ClearTimer` null "FireBP")
      (goto _label_2 :!via `Reset`))))

(event `FireBP`
  ;[1 1 1] Fire a Projectile
  (set `self.isOnCooldown` true)
  (for _ (range 1 (+ (`self.ProjectileAmountBP`) 1))
    (bind _output_get (set `self.MuzzleBP` (`SceneComponent.K2_GetComponentToWorld` (`self.MuzzleLocation`))))
    (bind _returnvalue (`self.AddInaccuracy` _output_get))
    (bind _returnvalue_2 (`|SpawnActorFromClass` "/Game/BP/Projectile_BP.Projectile_BP_C" _returnvalue "AlwaysSpawn" "OverrideRootScale"))
    ;;[1 1 1] Has bug of being destroyed before setting damage - do this before spawn via function
    (bind _output_get_2 (set `self.Projectile` _returnvalue_2))
    (set `/Game/BP/Projectile_BP.DamageBP` (`self.BulletDamage`) _output_get_2)))

(event `Cooldown`
  ;[1 1 1] Cooldown
  (`KismetSystemLibrary.Delay` (/ 1.0 (`self.RoundsPerSecondBP`)))
  (set `self.isOnCooldown` false))

(fn `UserConstructionScript`)